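; Player controller for a UE4-to-ROS bridge project that counts hits and triggers a reset once they pass a limit.
; HandleHit prints the count, increments it and compares it with MaxHitCount.
; Above the limit it zeroes the count, notifies the game mode's ROS bridge manager if valid, and has UE4ROSGameMode reset character poses.
; The event graph is inactive, holding only disconnected transform debug nodes.
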(event `self.ReceiveTick`
  (params (DeltaSeconds :type "Float (single-precision)")))

(fn `HandleHit`
  (bind _hitcount (`self.HitCount`))
  (`KismetSystemLibrary.PrintText` (`|FormatText` "Hit Count: {Count}" (`KismetTextLibrary.Conv_IntToText` _hitcount)))
  (bind _result (`/Engine/EditorBlueprintResources/StandardMacros.IncrementInt` _hitcount)
    (:`  `
      (`/Engine/EditorBlueprintResources/StandardMacros.CompareInt` _result (`self.MaxHitCount`)
        (:`>`
          (set `self.HitCount` 0)
          (bind _asue4rosgame_mode (cast `/UnrealCV/Blueprints/UE4ROSGameMode` (`GameplayStatics.GetGameMode`)))
          (bind _ue4rosbridgemanager (`/UnrealCV/Blueprints/UE4ROSGameMode.UE4ROSBridgeManager` _asue4rosgame_mode))
          (`/Engine/EditorBlueprintResources/StandardMacros.IsValid` _ue4rosbridgemanager
            (:`Is Valid`
              (`UE4ROSBridgeManager.HandleHit` _ue4rosbridgemanager))
            (:`Is Not Valid`
              _))
          (`/UnrealCV/Blueprints/UE4ROSGameMode.ResetCharacterPoses` _asue4rosgame_mode))))))

(fn `UserConstructionScript`)