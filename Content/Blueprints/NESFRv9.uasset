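; NESFRv9 is a player-controlled mobile robot pawn carrying a UR3 arm, linked to UE4ROSPlayerController.
; Input axes drive the base and rotate six arm joints, with the three wrist joints delegated to the UR3ForePart child actor.
; A zoomable camera attaches to that child's "camera"-tagged component, toggling with a third-person view.
; Body, RL and RR overlaps notify the controller; Move holds differential-force drive test code.
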(event `self.ReceiveBeginPlay`
  (`parent.ReceiveBeginPlay`)
  (`self.InitCamera`))

(event `self.ReceiveTick`
  (params (DeltaSeconds :type "Float (single-precision)"))
  (`parent.ReceiveTick` DeltaSeconds))

(event `InputAxis|MoveForward`
  (params (AxisValue :type "Float (single-precision)"))
  (`self.MoveForward` AxisValue))

(event `InputAxis|TurnRate`
  (params (AxisValue :type "Float (single-precision)"))
  (`self.TurnRight` AxisValue))

(event `InputAxis|RobotArm0`
  (params (AxisValue :type "Float (single-precision)"))
  (`SceneComponent.K2_AddLocalRotation` (`self.shoulder_pan_joint`) (`KismetMathLibrary.MakeRotator` 0.0 0.0 (* AxisValue (`GameplayStatics.GetWorldDeltaSeconds`) (`self.RobotArmMaxSpeed`))) false false))

(event `InputAxis|RobotArm1`
  (params (AxisValue :type "Float (single-precision)"))
  (`SceneComponent.K2_AddLocalRotation` (`self.shoulder_lift_joint`) (`KismetMathLibrary.MakeRotator` 0.0 (* AxisValue (`GameplayStatics.GetWorldDeltaSeconds`) (`self.RobotArmMaxSpeed`))) false false))

(event `InputAxis|RobotArm2`
  (params (AxisValue :type "Float (single-precision)"))
  (`SceneComponent.K2_AddLocalRotation` (`self.elbow_joint`) (`KismetMathLibrary.MakeRotator` 0.0 (* AxisValue (`GameplayStatics.GetWorldDeltaSeconds`) (`self.RobotArmMaxSpeed`))) false false))

(event `InputAxis|RobotArm3`
  (params (AxisValue :type "Float (single-precision)"))
  (bind _asur3fore_part (cast `/UnrealCV/Blueprints/UR3ForePart` (`ChildActorComponent.ChildActor` (`self.UR3ForePart`))))
  (`/UnrealCV/Blueprints/UR3ForePart.control_wrist_1_joint` _asur3fore_part (* AxisValue (`GameplayStatics.GetWorldDeltaSeconds`) (`self.RobotArmMaxSpeed`))))

(event `InputAxis|RobotArm4`
  (params (AxisValue :type "Float (single-precision)"))
  (bind _asur3fore_part (cast `/UnrealCV/Blueprints/UR3ForePart` (`ChildActorComponent.ChildActor` (`self.UR3ForePart`))))
  (`/UnrealCV/Blueprints/UR3ForePart.control_wrist_2_joint` _asur3fore_part (* AxisValue (`GameplayStatics.GetWorldDeltaSeconds`) (`self.RobotArmMaxSpeed`))))

(event `InputAxis|RobotArm5`
  (params (AxisValue :type "Float (single-precision)"))
  (bind _asur3fore_part (cast `/UnrealCV/Blueprints/UR3ForePart` (`ChildActorComponent.ChildActor` (`self.UR3ForePart`))))
  (`/UnrealCV/Blueprints/UR3ForePart.control_wrist_3_joint` _asur3fore_part (* AxisValue (`GameplayStatics.GetWorldDeltaSeconds`) (`self.RobotArmMaxSpeed`))))

(event `Key|C`
  (params (Key :type "Key Structure"))
  (bind _3rdviewcamera (`self.3rdViewCamera`))
  (bind _camera (`self.Camera`))
  (:`Pressed`
    (`/Engine/EditorBlueprintResources/StandardMacros.FlipFlop`
      (:`A`
        (`ActorComponent.SetActive` _3rdviewcamera true false)
        (`ActorComponent.SetActive` _camera false false))
      (:`B`
        (`ActorComponent.SetActive` _camera true false)
        (`ActorComponent.SetActive` _3rdviewcamera false false)))))

(event `InputAxis|Zoom`
  (params (AxisValue :type "Float (single-precision)"))
  (bind _camera (`self.Camera`))
  (bind _returnvalue (`KismetMathLibrary.FClamp` (+ (* AxisValue 1.0) (`CameraComponent.FieldOfView` _camera)) 10.0 120.0))
  (`KismetSystemLibrary.PrintString` (`KismetStringLibrary.Conv_DoubleToString` _returnvalue) false false)
  (`CameraComponent.SetFieldOfView` _camera _returnvalue))

(event `self.ReceiveHit`
  (params (MyComp :type "PrimitiveComponent Object Reference") (Other :type "Actor Object Reference") (OtherComp :type "PrimitiveComponent Object Reference") (bSelfMoved :type Boolean) (HitLocation :type "Vector Structure") (HitNormal :type "Vector Structure") (NormalImpulse :type "Vector Structure") (Hit :type "HitResult Structure (by ref)")))

(event `self.RootBody.OnComponentBeginOverlap`
  (params (OverlappedComponent :type "PrimitiveComponent Object Reference") (OtherActor :type "Actor Object Reference") (OtherComp :type "PrimitiveComponent Object Reference") (OtherBodyIndex :type Integer) (bFromSweep :type Boolean) (SweepResult :type "HitResult Structure (by ref)"))
  (`|ExecutionSequence`
    (:`then_0`
      (`KismetSystemLibrary.PrintText` (`|FormatText` "Hit NESFRv9 {MyComp}, {Other}, {OtherComp}" (`KismetTextLibrary.Conv_StringToText` (`KismetSystemLibrary.GetDisplayName` OverlappedComponent)) (`KismetTextLibrary.Conv_StringToText` (`KismetSystemLibrary.GetDisplayName` OtherActor)) (`KismetTextLibrary.Conv_StringToText` (`KismetSystemLibrary.GetDisplayName` OtherComp)))))
    (:`then_1`
      (`KismetSystemLibrary.PrintString` "HITBEGIN" :!label _label)
      (bind _asue4rosplayer_controller (cast `/UnrealCV/Blueprints/UE4ROSPlayerController` (`self.GetController`)))
      (`/UnrealCV/Blueprints/UE4ROSPlayerController.HandleOverlap` _asue4rosplayer_controller)
      (`KismetSystemLibrary.PrintString` "HITEND"))))

(event `self.RL.OnComponentBeginOverlap`
  (params (OverlappedComponent :type "PrimitiveComponent Object Reference") (OtherActor :type "Actor Object Reference") (OtherComp :type "PrimitiveComponent Object Reference") (OtherBodyIndex :type Integer) (bFromSweep :type Boolean) (SweepResult :type "HitResult Structure (by ref)"))
  (goto _label))

(event `self.RR.OnComponentBeginOverlap`
  (params (OverlappedComponent :type "PrimitiveComponent Object Reference") (OtherActor :type "Actor Object Reference") (OtherComp :type "PrimitiveComponent Object Reference") (OtherBodyIndex :type Integer) (bFromSweep :type Boolean) (SweepResult :type "HitResult Structure (by ref)"))
  (goto _label))

(event `self.RootBody.OnComponentEndOverlap`
  (params (OverlappedComponent :type "PrimitiveComponent Object Reference") (OtherActor :type "Actor Object Reference") (OtherComp :type "PrimitiveComponent Object Reference") (OtherBodyIndex :type Integer))
  ;[1 1 1] DebugTest
)

(event `self.Shoulder_Link.OnComponentBeginOverlap`
  (params (OverlappedComponent :type "PrimitiveComponent Object Reference") (OtherActor :type "Actor Object Reference") (OtherComp :type "PrimitiveComponent Object Reference") (OtherBodyIndex :type Integer) (bFromSweep :type Boolean) (SweepResult :type "HitResult Structure (by ref)"))
  ;[1 1 1] DebugTest
  (`KismetSystemLibrary.PrintString` (`KismetSystemLibrary.GetDisplayName` OverlappedComponent))
  (`KismetSystemLibrary.PrintString` (`KismetSystemLibrary.GetDisplayName` OtherComp)))

(event `self.UpperArm_Link.OnComponentBeginOverlap`
  (params (OverlappedComponent :type "PrimitiveComponent Object Reference") (OtherActor :type "Actor Object Reference") (OtherComp :type "PrimitiveComponent Object Reference") (OtherBodyIndex :type Integer) (bFromSweep :type Boolean) (SweepResult :type "HitResult Structure (by ref)"))
  ;[1 1 1] DebugTest
)

(event `self.elbow_joint.OnComponentBeginOverlap`
  (params (OverlappedComponent :type "PrimitiveComponent Object Reference") (OtherActor :type "Actor Object Reference") (OtherComp :type "PrimitiveComponent Object Reference") (OtherBodyIndex :type Integer) (bFromSweep :type Boolean) (SweepResult :type "HitResult Structure (by ref)"))
  ;[1 1 1] DebugTest
  (`KismetSystemLibrary.PrintString` (`KismetSystemLibrary.GetDisplayName` OverlappedComponent))
  (`KismetSystemLibrary.PrintString` (`KismetSystemLibrary.GetDisplayName` OtherComp)))

(fn `InitCamera`
  (`ActorComponent.SetActive` (`self.Camera`) false false)
  (`ActorComponent.SetActive` (`self.RGBDCamRGB`) false false)
  (`ActorComponent.SetActive` (`self.RGBDCamDepth`) false false)
  (`ActorComponent.SetActive` (`self.3rdViewCamera`) true false)
  ;[1 1 1] Workaround Forced-Locate Camera
  (`SceneComponent.K2_SetRelativeLocation` (`self.Camera`) (0.0 0.0 0.0) false false))

(fn `Move`
  (params (Direction :type "Vector Structure"))
  (bind _returnvalue (`KismetMathLibrary.Normal` Direction))
  (bind _rootbody (`self.RootBody`))
  (bind _maxdriveforce (`self.MaxDriveForce`))
  (bind _returnvalue_2 (`KismetMathLibrary.Dot_VectorVector` _returnvalue (`self.LocalForwardVector`)))
  (bind _returnvalue_3 (`KismetMathLibrary.Dot_VectorVector` _returnvalue (`self.LocalRightVector`)))
  ;[1 1 1] TestCode for PhysicsConstraint-Based Robot Movement
  (`|ExecutionSequence`
    (:`then_0`
      (`PrimitiveComponent.AddForceAtLocationLocal` _rootbody (`KismetMathLibrary.MakeVector` (* (+ _returnvalue_2 _returnvalue_3) _maxdriveforce) 0.0 -10.0) (0.0 -25.0 20.0) "None"))
    (:`then_1`
      (`PrimitiveComponent.AddForceAtLocationLocal` _rootbody (`KismetMathLibrary.MakeVector` (* (- _returnvalue_2 _returnvalue_3) _maxdriveforce) 0.0 -10.0) (0.0 25.0 20.0) "None"))))

(fn `UserConstructionScript`
  (`parent.UserConstructionScript`)
  (`|ExecutionSequence`
    (:`then_0`
      (for _array_element (`self.GetComponentsByTag` (`ChildActorComponent.ChildActor` (`self.UR3ForePart`)) "/Script/Engine.SceneComponent" "camera")
        (`SceneComponent.K2_AttachToComponent` (`self.Camera`) _array_element "None" "KeepRelative" "KeepRelative" "KeepRelative" true)))))