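; Blueprint for the forearm section of a robot arm, apparently a UR3, that lets the player drive its three wrist joints.
; Three input axes, RobotArm3 to RobotArm5, each feed a function that adds the raw axis value as local rotation to one wrist component.
; Wrists 1 and 3 turn in pitch and wrist 2 in yaw, all teleported, with no delta-time scaling or joint limits.
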(event `InputAxis|RobotArm3`
  (params (AxisValue :type "Float (single-precision)"))
  (`self.control_wrist_1_joint` AxisValue))

(event `InputAxis|RobotArm4`
  (params (AxisValue :type "Float (single-precision)"))
  (`self.control_wrist_2_joint` AxisValue))

(event `InputAxis|RobotArm5`
  (params (AxisValue :type "Float (single-precision)"))
  (`self.control_wrist_3_joint` AxisValue))

(fn `control_wrist_1_joint`
  (params (value :type "Float (double-precision)"))
  (`SceneComponent.K2_AddLocalRotation` (`self.wrist_1_joint`) (`KismetMathLibrary.MakeRotator` 0.0 value) false true))

(fn `control_wrist_2_joint`
  (params (value :type "Float (double-precision)"))
  (`SceneComponent.K2_AddLocalRotation` (`self.wrist_2_joint`) (`KismetMathLibrary.MakeRotator` 0.0 0.0 value) false true))

(fn `control_wrist_3_joint`
  (params (value :type "Float (double-precision)"))
  (`SceneComponent.K2_AddLocalRotation` (`self.wrist_3_joint`) (`KismetMathLibrary.MakeRotator` 0.0 value) false true))

(fn `UserConstructionScript`)