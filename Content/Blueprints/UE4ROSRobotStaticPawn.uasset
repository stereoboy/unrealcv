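; A ROS robot pawn that moves by rewriting its actor transform each tick rather than using physics.
; MoveForward and TurnRight store a vector and rotator, which Tick scales by base speeds and delta time and composes in local space, without sweep.
; LookUp and LookRight axes rotate the Altitude and Azimuth components for a third-person camera.
; ResetPose teleports back to the BeginPlay transform and realigns the controller's rotation.
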(event `self.ReceiveBeginPlay`
  (bind _output_get (set `self.InitialPose` (`self.GetTransform`)))
  (`KismetSystemLibrary.PrintString` (`KismetStringLibrary.Conv_TransformToString` _output_get) true true (struct :`R` 1.0 :`B` 0.845811 :`A` 1.0)))

(event `self.ReceiveTick`
  (params (DeltaSeconds :type "Float (single-precision)"))
  (`parent.ReceiveTick` DeltaSeconds)
  (`self.K2_SetActorTransform` (`KismetMathLibrary.ComposeTransforms` (`KismetMathLibrary.MakeTransform` (* (`self.MoveForwardVector`) (* DeltaSeconds (`self.MoveForwardBaseSpeed`))) (* (`self.TurnRightRotator`) (* DeltaSeconds (`self.TurnRightBaseSpeed`)))) (`self.GetTransform`))))

(event `self.ResetPose`
  (`self.ResetPoseImpl`))

(event `InputAxis|LookUp`
  (params (AxisValue :type "Float (single-precision)"))
  (`SceneComponent.K2_AddLocalRotation` (`self.Altitude`) (`KismetMathLibrary.MakeRotator` 0.0 (* AxisValue 10.0)) false false))

(event `InputAxis|LookRight`
  (params (AxisValue :type "Float (single-precision)"))
  (`SceneComponent.K2_AddLocalRotation` (`self.Azimuth`) (`KismetMathLibrary.MakeRotator` 0.0 0.0 (* AxisValue 10.0)) false false))

(fn `MoveForward`
  (params (AxisValue :type "Float (double-precision)"))
  (set `self.MoveForwardVector` (`KismetMathLibrary.MakeVector` (* AxisValue 1.0))))

(fn `ResetPoseImpl`
  (bind _returnvalue (`self.GetController`))
  (bind _initialpose (`self.InitialPose`))
  (`self.K2_SetActorTransform` _initialpose false true)
  (`/Engine/EditorBlueprintResources/StandardMacros.IsValid` _returnvalue
    (:`Is Valid`
      (`Controller.SetControlRotation` _returnvalue (`KismetMathLibrary.TransformRotation` _initialpose))
      (`KismetSystemLibrary.PrintString` (`KismetStringLibrary.Conv_TransformToString` _initialpose) true true (struct :`R` 1.0 :`B` 0.9625 :`A` 1.0) 15.0))))

(fn `TurnRight`
  (params (AxisValue :type "Float (double-precision)"))
  (set `self.TurnRightRotator` (`KismetMathLibrary.MakeRotator` 0.0 0.0 (* AxisValue 1.0))))

(fn `UserConstructionScript`)