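; UE4ROSRobot is a controllable robot Blueprint with a third-person view camera and a pose reset.
; BeginPlay stores and prints the starting transform, which the ResetPose event restores through ResetPoseImpl.
; The reset also realigns the controller's control rotation to that pose and prints it.
; LookUp and LookRight axis inputs orbit the view by adding scaled local pitch to Altitude and yaw to Azimuth.
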(event `self.ReceiveBeginPlay`
  (bind _output_get (set `self.InitialPose` (`self.GetTransform`)))
  (`KismetSystemLibrary.PrintString` (`KismetStringLibrary.Conv_TransformToString` _output_get) true true (struct :`R` 1.0 :`B` 0.845811 :`A` 1.0)))

(event `self.ResetPose`
  (`self.ResetPoseImpl`))

(event `InputAxis|LookUp`
  (params (AxisValue :type "Float (single-precision)"))
  (`SceneComponent.K2_AddLocalRotation` (`self.Altitude`) (`KismetMathLibrary.MakeRotator` 0.0 (* AxisValue 10.0)) false false))

(event `InputAxis|LookRight`
  (params (AxisValue :type "Float (single-precision)"))
  (`SceneComponent.K2_AddLocalRotation` (`self.Azimuth`) (`KismetMathLibrary.MakeRotator` 0.0 0.0 (* AxisValue 10.0)) false false))

(fn `ResetPoseImpl`
  (bind _initialpose (`self.InitialPose`))
  (`self.K2_SetActorTransform` _initialpose)
  (`Controller.SetControlRotation` (`self.GetController`) (`KismetMathLibrary.TransformRotation` _initialpose))
  (`KismetSystemLibrary.PrintString` (`KismetStringLibrary.Conv_TransformToString` _initialpose) true true (struct :`R` 1.0 :`B` 0.9625 :`A` 1.0) 15.0))

(fn `UserConstructionScript`)