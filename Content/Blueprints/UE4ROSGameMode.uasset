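; UE4ROSGameMode is a game mode Blueprint that manages the connection between the game and ROS through a UE4ROSBridgeManager actor.
; ToggleConnectUE4ROS destroys the existing manager, or spawns one at the origin and attaches its capture component to the first player pawn's camera.
; The manager's validity serves as the connection state, which IsConnected reports.
; BeginPlay is empty, and the windowed-resolution and PublishReward nodes are left unwired.
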(event `self.ReceiveBeginPlay`)

(fn `IsConnected`
  (returns (ReturnValue :type Boolean))
  (return (`KismetSystemLibrary.IsValid` (`self.UE4ROSBridgeManager`))))

(fn `ToggleConnectUE4ROS`
  (bind _ue4rosbridgemanager (`self.UE4ROSBridgeManager`))
  (`/Engine/EditorBlueprintResources/StandardMacros.IsValid` _ue4rosbridgemanager
    (:`Is Valid`
      ;[1 1 1] Disconnect
      (`self.K2_DestroyActor` _ue4rosbridgemanager))
    (:`Is Not Valid`
      ;[1 1 1] Connect
      (bind _returnvalue (`|SpawnActorFromClass` "/Script/UnrealCV.UE4ROSBridgeManager" (`KismetMathLibrary.MakeTransform` (0.0 0.0 0.0)) "Undefined" "OverrideRootScale" null null))
      (bind _output_get (set `self.UE4ROSBridgeManager` _returnvalue))
      (`UE4ROSBridgeManager.AttachCaptureComponentToCamera` _output_get (`GameplayStatics.GetPlayerPawn` 0)))))

(fn `UserConstructionScript`
  (locals (NewLocalVar_0 :type Integer)))