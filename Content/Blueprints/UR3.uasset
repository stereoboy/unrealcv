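; UR3 robot arm Blueprint that lets the player jog each of its six joints directly through input axes.
; Each RobotArm axis calls its own control function for shoulder pan, shoulder lift, elbow or one of three wrist joints.
; Those functions add the raw axis value as local yaw or pitch to the joint component, with no limits or delta-time scaling.
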(event `InputAxis|RobotArm0`
  (params (AxisValue :type "Float (single-precision)"))
  (`self.control_shoulder_pan_joint` AxisValue))

(event `InputAxis|RobotArm1`
  (params (AxisValue :type "Float (single-precision)"))
  (`self.control_shoulder_lift_joint` AxisValue))

(event `InputAxis|RobotArm2`
  (params (AxisValue :type "Float (single-precision)"))
  (`self.control_elbow_joint` AxisValue))

(event `InputAxis|RobotArm3`
  (params (AxisValue :type "Float (single-precision)"))
  (`self.control_wrist_1_joint` AxisValue))

(event `InputAxis|RobotArm4`
  (params (AxisValue :type "Float (single-precision)"))
  (`self.control_wrist_2_joint` AxisValue))

(event `InputAxis|RobotArm5`
  (params (AxisValue :type "Float (single-precision)"))
  (`self.control_wrist_3_joint` AxisValue))

(fn `control_elbow_joint`
  (params (value :type "Float (double-precision)"))
  (`SceneComponent.K2_AddLocalRotation` (`self.elbow_joint`) (`KismetMathLibrary.MakeRotator` 0.0 value) false false))

(fn `control_shoulder_lift_joint`
  (params (value :type "Float (double-precision)"))
  (`SceneComponent.K2_AddLocalRotation` (`self.shoulder_lift_joint`) (`KismetMathLibrary.MakeRotator` 0.0 value) false false))

(fn `control_shoulder_pan_joint`
  (params (value :type "Float (double-precision)"))
  (`SceneComponent.K2_AddLocalRotation` (`self.shoulder_pan_joint`) (`KismetMathLibrary.MakeRotator` 0.0 0.0 value) false false))

(fn `control_wrist_1_joint`
  (params (value :type "Float (double-precision)"))
  (`SceneComponent.K2_AddLocalRotation` (`self.wrist_1_joint`) (`KismetMathLibrary.MakeRotator` 0.0 value) false false))

(fn `control_wrist_2_joint`
  (params (value :type "Float (double-precision)"))
  (`SceneComponent.K2_AddLocalRotation` (`self.wrist_2_joint`) (`KismetMathLibrary.MakeRotator` 0.0 0.0 value) false false))

(fn `control_wrist_3_joint`
  (params (value :type "Float (double-precision)"))
  (`SceneComponent.K2_AddLocalRotation` (`self.wrist_3_joint`) (`KismetMathLibrary.MakeRotator` 0.0 value) false false))

(fn `UserConstructionScript`)